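; GM_TP2 is the game mode for the TP2 level, ending it when the player collects enough chests and coins.
; After a short delay on BeginPlay it caches the first player's BP_TP2PlayerState and binds CheckVictory to its OnCountersChanged event.
; CheckVictory compares the chest and coin counts to the required totals, then prints a completion message and pauses the game.
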(event Custom|CheckVictory
  (bind _playerstateref (Variables|Default|GetPlayerStateRef))
  (if (and (>= (Variables|/Game/level/TP2/BP_TP2PlayerState.BP_TP2PlayerState_C|GetChestCount _playerstateref) (Variables|Default|GetRequiredChests)) (>= (Variables|/Game/level/TP2/BP_TP2PlayerState.BP_TP2PlayerState_C|GetCoinCount _playerstateref) (Variables|Default|GetRequiredCoins)))
    (Development|PrintString "LEVEL COMPLETE" true true "(R=0.000000,G=0.660000,B=1.000000,A=1.000000)" 1e+01)
    (Game|SetGamePaused true)))

(event EventBeginPlay
  (Utilities|FlowControl|Delay 0.2)
  (bind _asbp_tp2player_state (Utilities|Casting|CastToBP_TP2PlayerState (Game|GetPlayerState 0)))
  (bind _output_get (Variables|Default|SetPlayerStateRef _asbp_tp2player_state))
  (EventDispatchers|BindEventtoOnCountersChanged _output_get (delegate Custom|CheckVictory)))

(fn ConstructionScript)