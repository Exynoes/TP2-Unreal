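; BP_TP2PlayerState is the player state for the TP2 level, holding the player's chest and coin counters.
; AddChest and AddCoin each increment their counter, print a value to the screen and fire the OnCountersChanged dispatcher so listeners can react.
; The event graph and construction script are empty, so all logic lives in those two functions.
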(event EventBeginPlay)

(event EventTick
  (params (DeltaSeconds :type Float%20%28single-precision%29)))

(fn ConstructionScript)

(fn AddChest
  (bind _result (Math|Integer|IncrementInt (Variables|Default|GetChestCount))
    (:%20%20
      (Development|PrintString (Utilities|String|ToString(Integer) _result))
      (Default|CallOnCountersChanged))))

(fn AddCoin
  (bind _result (Math|Integer|IncrementInt (Variables|Default|GetCoinCount))
    (:%20%20
      (Development|PrintString (Utilities|String|ToString(Integer) _result))
      (Default|CallOnCountersChanged))))