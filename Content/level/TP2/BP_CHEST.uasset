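; BP_CHEST is an interactable chest in the TP2 level that opens once and counts toward the player's chest tally.
; On Interact, an IsOpen guard blocks repeat use, then it calls AddChest on the first player's BP_TP2PlayerState.
; A timeline then swings the lid by lerping the LidPivot roll from zero to OpenAngle.
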(event EventBeginPlay)

(event Collision|EventActorBeginOverlap
  (params (OtherActor :type Actor%20Object%20Reference)))

(event EventTick
  (params (DeltaSeconds :type Float%20%28single-precision%29)))

(event EventInteract
  (if (not (Variables|Default|GetIsOpen))
    (Variables|Default|SetIsOpen true)
    (bind _asbp_tp2player_state (Utilities|Casting|CastToBP_TP2PlayerState (Game|GetPlayerState 0)))
    (Default|AddChest _asbp_tp2player_state)
    (bind _alpha (Timeline|Timeline PlayFromStart)
      (:Update
        (Transformation|SetRelativeRotation (Variables|Default|GetLidPivot) (Math|Rotator|MakeRotator (Math|Float|Lerp 0.0 (Variables|Default|GetOpenAngle) _alpha) 0.0 0.0) false false)))))

(fn ConstructionScript)